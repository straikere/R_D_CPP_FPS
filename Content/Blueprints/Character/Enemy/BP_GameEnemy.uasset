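; BP_GameEnemy is an enemy that shows an alert-level indicator when the first-person player is nearby.
; Its Sphere overlap events filter for BP_FirstPersonCharacter, then call Show or Hide on the WBP_AlertLevel inside its widget component.
; A DrawSIze helper sets the widget's draw size, but DistanceReDraw is an unfinished stub whose call to it never runs.
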(event OnComponentBeginOverlap(Sphere)
  (params (OverlappedComponent :type Primitive%20Component%20Object%20Reference) (OtherActor :type Actor%20Object%20Reference) (OtherComp :type Primitive%20Component%20Object%20Reference) (OtherBodyIndex :type Integer) (bFromSweep :type Boolean) (SweepResult :type Hit%20Result%20Structure%20%28by%20ref%29))
  (Utilities|Casting|CastToBP_FirstPersonCharacter OtherActor)
  (bind _aswbp_alert_level (Utilities|Casting|CastToWBP_AlertLevel (UserInterface|GetWidget (Variables|Default|GetWBP_AlertLevel))))
  (Default|Show _aswbp_alert_level))

(event OnComponentEndOverlap(Sphere)
  (params (OverlappedComponent :type Primitive%20Component%20Object%20Reference) (OtherActor :type Actor%20Object%20Reference) (OtherComp :type Primitive%20Component%20Object%20Reference) (OtherBodyIndex :type Integer))
  (Utilities|Casting|CastToBP_FirstPersonCharacter OtherActor)
  (bind _aswbp_alert_level (Utilities|Casting|CastToWBP_AlertLevel (UserInterface|GetWidget (Variables|Default|GetWBP_AlertLevel))))
  (Default|Hide _aswbp_alert_level))

(event EventBeginPlay)

(event Collision|EventActorBeginOverlap
  (params (OtherActor :type Actor%20Object%20Reference)))

(event EventTick
  (params (DeltaSeconds :type Float%20%28single-precision%29)))

(fn ConstructionScript)

(fn DrawSIze
  (params (Size :type Vector%202D%20Structure))
  (Class|WidgetComponent|SetDrawSize (Variables|Default|GetWBP_AlertLevel) Size))

(fn DistanceReDraw)