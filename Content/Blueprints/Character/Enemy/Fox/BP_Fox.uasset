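; BP_Fox is a fox enemy character with a run toggle and a head-based melee attack.
; Run swaps in boosted speed and acceleration or restores original acceleration, opening a Tick-driven gate that sets walk speed via FInterpTo toward the original.
; Attack passes a gate to sphere-trace forward from the head socket, applying a GAS instant damage effect to a hit Character's PlayerState.
; A successful hit closes that gate until a three-second cooldown timer reopens it.
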(event Custom|Run
  (params (Run :type Boolean))
  (bind _charactermovement (Variables|Character|GetCharacterMovement))
  (bind _charactermovement_2 (Variables|Character|GetCharacterMovement))
  (bind _max_walk_speed (Variables|Default|GetMax%20Walk%20Speed))
  (bind _output_get (Variables|Default|SetRun_0 Run))
  (Development|PrintString (Utilities|String|ToString(Boolean) _output_get) true false "(R=0.000000,G=0.660000,B=1.000000,A=1.000000)" 2.0 "2")
  (if _output_get
    (Variables|/Script/Engine.CharacterMovementComponent|SetMaxAcceleration _charactermovement_2 (Variables|Default|GetMax%20Acceleration))
    (Variables|/Script/Engine.CharacterMovementComponent|SetMaxWalkSpeed _charactermovement_2 _max_walk_speed)
    (else
      (Utilities|FlowControl|DoOnce false
        (:Completed
          (Variables|/Script/Engine.CharacterMovementComponent|SetMaxAcceleration _charactermovement (Variables|Default|GetOrig%20Max%20Acceleration))
          (Utilities|FlowControl|Gate true) ; enters at Open
        )))))

(event Custom|Attack
  (bind _mesh (Variables|Character|GetMesh))
  (bind _returnvalue (Transformation|GetSocketLocation _mesh "Fox_-HeadSocket"))
  (Utilities|FlowControl|Gate false :!label _label
    (:Exit
      (bind _outhit (Collision|SphereTraceByChannel _returnvalue (+ _returnvalue (* (Math|Vector|GetForwardVector (Transformation|GetSocketRotation _mesh "Fox_-HeadSocket")) 7e+01)) 2e+01 "TraceTypeQuery1" false 0 "ForDuration"))
      (if (.bBlockingHit (Collision|BreakHitResult _outhit))
        (bind _ascharacter (Utilities|Casting|CastToCharacter (.HitActor (Collision|BreakHitResult _outhit))))
        (GameplayEffects|ApplyGameplayEffectToSelf :self (Ability|GetAbilitySystemComponent (Variables|/Script/Engine.Pawn|GetPlayerState _ascharacter)) :GameplayEffectClass "/Game/GameplayEffects/Damage/GE_InstantDamage.GE_InstantDamage_C")
        (Utilities|Time|SetTimerbyEvent (delegate Custom|OpenAttac) 3.0)
        (goto _label Close)))))

(event Custom|OpenAttac
  (bind _mesh (Variables|Character|GetMesh))
  (bind _returnvalue (Transformation|GetSocketLocation _mesh "Fox_-HeadSocket"))
  (Utilities|FlowControl|Gate false) ; enters at Open
)

(event EventBeginPlay
  (bind _charactermovement (Variables|Character|GetCharacterMovement))
  (Variables|Default|SetOrig%20Max%20Walk%20Speed (Variables|/Script/Engine.CharacterMovementComponent|GetMaxWalkSpeed _charactermovement))
  (Variables|Default|SetOrig%20Max%20Acceleration (Variables|/Script/Engine.CharacterMovementComponent|GetMaxAcceleration _charactermovement))
  (Components|Activation|Deactivate (Variables|Default|GetNiagara1)))

(event Collision|EventActorBeginOverlap
  (params (OtherActor :type Actor%20Object%20Reference)))

(event EventTick
  (params (DeltaSeconds :type Float%20%28single-precision%29))
  (bind _charactermovement (Variables|Character|GetCharacterMovement))
  (Utilities|FlowControl|Gate true
    (:Exit
      (Variables|/Script/Engine.CharacterMovementComponent|SetMaxWalkSpeed _charactermovement (Math|Interpolation|FInterpTo (Variables|Default|GetMax%20Walk%20Speed) (Variables|Default|GetOrig%20Max%20Walk%20Speed) DeltaSeconds 0.5))
      (Utilities|FlowControl|Delay 0.2)
      (Utilities|FlowControl|DoOnce false) ; enters at Reset
    )))

(fn ConstructionScript
  (|CallParentFunction))