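; Base interactable actor that is either picked up (prints a message and destroys itself) or opens a crafting widget.
; Highlight shows an info widget filled by item tag, turns on custom depth stencil and enables the actor's own input for interact and destroy actions.
; Interacting with non-pickables blocks movement and switches to UI-only input.
; UnHighlight reverses highlighting and closes crafting; movement returns after a short delay.
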(event Custom|Destoyed_Event
  (Utilities|FlowControl|Delay 0.2)
  (Input|ResetIgnoreMoveInput (Variables|Default|GetAs%20Player%20Controller)))

(event Input|EnhancedActionEvents|EnhancedInputActionIA_Interaction
  (params (ActionValue :type Boolean) (ElapsedSeconds :type Float%20%28double-precision%29) (TriggeredSeconds :type Float%20%28double-precision%29) (InputAction :type Input%20Action%20Object%20Reference :default "/Game/Blueprints/Input/IA/IA_Interaction.IA_Interaction"))
  (bind _as_player_controller (Variables|Default|GetAs%20Player%20Controller))
  (if (Variables|Default|GetIsPickable)
    (Development|PrintString (Utilities|String|Append "You picked Up: " (Utilities|GetClassDisplayName (Utilities|GetClass self))))
    (Actor|DestroyActor)
    (else
      (Input|SetIgnoreMoveInput _as_player_controller true)
      (Variables|/Script/Engine.PlayerController|SetbShowMouseCursor _as_player_controller true)
      (Input|SetInputModeUIOnly _as_player_controller 0 "DoNotLock" false)
      (bind _returnvalue (UserInterface|CreateWidget "/Game/UI_FOR_TESTS/WBP_Crafting.WBP_Crafting_C" _as_player_controller))
      (bind _output_get (Variables|Default|SetCraftWidget _returnvalue))
      (EventDispatchers|AssignDestoyed _output_get (delegate Custom|Destoyed_Event))
      (UserInterface|Viewport|AddtoViewport _output_get 0))))

(event Input|EnhancedActionEvents|EnhancedInputActionIA_Destroy
  (params (ActionValue :type Boolean) (ElapsedSeconds :type Float%20%28double-precision%29) (TriggeredSeconds :type Float%20%28double-precision%29) (InputAction :type Input%20Action%20Object%20Reference :default "/Game/Blueprints/Input/IA/IA_Destroy.IA_Destroy"))
  (Actor|DestroyActor))

(event EventBeginPlay
  (CallFunction|SetVisibilitys "Hidden")
  (Default|SetInfo (.AsWBP%20Info (Utilities|Casting|CastToWBP_Info (UserInterface|GetWidget (Variables|Default|GetWidget)))) (Class|ItemInfo|FindItemInfoforTag (Variables|Default|GetItemInfo) (Variables|Default|GetItemTag))))

(event EventHighlight
  (params (Inicigator :type BP%20First%20Person%20Character%20Object%20Reference))
  (bind _returnvalue (Pawn|GetController Inicigator))
  (bind _staticmesh (Variables|Default|GetStaticMesh))
  (bind (_asplayer_controller _bsuccess) (Utilities|Casting|CastToPlayerController _returnvalue))
  (CallFunction|SetVisibilitys "Visible")
  (Rendering|SetRenderCustomDepth _staticmesh true)
  (Rendering|SetCustomDepthStencilValue _staticmesh (Variables|Default|GetCustomDepthValue))
  (if _bsuccess
    (Variables|Default|SetAs%20Player%20Controller _asplayer_controller)
    (Input|EnableInput _asplayer_controller)))

(event EventUnHighlight
  (CallFunction|SetVisibilitys "Hidden")
  (Rendering|SetRenderCustomDepth (Variables|Default|GetStaticMesh) false)
  (if (Variables|Default|GetIsPickable)
    (Input|DisableInput (Variables|Default|GetAs%20Player%20Controller))
    (else
      (Utilities|FlowControl|Sequence
        (:then_0
          (Variables|Default|GetAs%20Player%20Controller
            (:then
              (Input|DisableInput (Variables|Default|GetAs%20Player%20Controller))
              (Utilities|FlowControl|Delay 0.2)
              (Input|ResetIgnoreMoveInput (Variables|Default|GetAs%20Player%20Controller)))
            (:else)))
        (:then_1
          (bind _craftwidget (Variables|Default|GetCraftWidget)
            (:then
              (Default|Destroy _craftwidget))
            (:else)))))))

(fn ConstructionScript)

(fn SetVisibilitys
  (params (InVisibility :type ESlateVisibility%20Enum :default "Visible"))
  (Widget|SetVisibility (UserInterface|GetWidget (Variables|Default|GetWidget)) InVisibility))