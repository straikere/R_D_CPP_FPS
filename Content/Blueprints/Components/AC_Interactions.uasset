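; Actor component for the first-person character, meant to detect and highlight interactable actors in view.
; It caches the owning character on BeginPlay and runs a Visibility line trace every Tick, casting the hit to BP_InteractActorBase.
; The logic tracking last and current actors to toggle Highlight and UnHighlight is disconnected.
; CameraPosition's camera-forward offset calculation is also unused, so the component currently has no visible effect.
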(event EventBeginPlay
  (bind _asbp_first_person_character (Utilities|Casting|CastToBP_FirstPersonCharacter (Components|GetOwner)))
  (Variables|Default|SetBP%20First%20Person%20Character _asbp_first_person_character))

(event EventTick
  (params (DeltaSeconds :type Float%20%28single-precision%29))
  (CallFunction|InteractTrace))

(fn InteractTrace
  (bind (_start _end) (|CameraPosition))
  (bind _outhit (Collision|LineTraceByChannel _start _end "TraceTypeQuery1" false 0 "None"))
  (Utilities|Casting|CastToBP_InteractActorBase (.HitActor (Collision|BreakHitResult _outhit))))