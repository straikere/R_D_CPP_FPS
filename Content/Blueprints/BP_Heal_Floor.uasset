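; BP_Heal_Floor is a floor zone that applies the GE_Heal gameplay effect to characters standing inside its box.
; Box begin overlap applies the effect through the Ability System Component on the character's PlayerState and stores the returned handle.
; End overlap removes the effect by that handle.
; A single handle variable serves all characters, so each new entry overwrites the previous one.
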(event OnComponentBeginOverlap(Box)
  (params (OverlappedComponent :type Primitive%20Component%20Object%20Reference) (OtherActor :type Actor%20Object%20Reference) (OtherComp :type Primitive%20Component%20Object%20Reference) (OtherBodyIndex :type Integer) (bFromSweep :type Boolean) (SweepResult :type Hit%20Result%20Structure%20%28by%20ref%29))
  (bind _ascharacter (Utilities|Casting|CastToCharacter OtherActor))
  (bind _returnvalue (GameplayEffects|ApplyGameplayEffectToSelf :self (Ability|GetAbilitySystemComponent (Variables|/Script/Engine.Pawn|GetPlayerState _ascharacter)) :GameplayEffectClass "/Game/GameplayEffects/GE_Heal.GE_Heal_C"))
  (Variables|Default|SetDamageZoneEffect _returnvalue))

(event OnComponentEndOverlap(Box)
  (params (OverlappedComponent :type Primitive%20Component%20Object%20Reference) (OtherActor :type Actor%20Object%20Reference) (OtherComp :type Primitive%20Component%20Object%20Reference) (OtherBodyIndex :type Integer))
  (bind _ascharacter (Utilities|Casting|CastToCharacter OtherActor))
  (Utilities|IsValid (Ability|GetAbilitySystemComponent (Variables|/Script/Engine.Pawn|GetPlayerState _ascharacter))
    (:Is%20Valid
      (GameplayEffects|RemoveActiveGameplayEffect (Ability|GetAbilitySystemComponent (Variables|/Script/Engine.Pawn|GetPlayerState _ascharacter)) (Variables|Default|GetDamageZoneEffect) -1))))

(fn ConstructionScript)