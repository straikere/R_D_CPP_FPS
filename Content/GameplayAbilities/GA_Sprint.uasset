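; Gameplay ability that lets a character sprint by raising max walk speed to RunSpeed while input is held.
; Activation caches the base speed, requires horizontal velocity above a threshold, and must commit successfully.
; Input release ends the ability, while a Gameplay.CancelSprint event cancels it.
; OnEndAbility removes owner effects with the Ability.Sprint asset tag and restores the cached speed.
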(event Ability|EventActivateAbility
  (bind _ascharacter (Utilities|Casting|CastToCharacter (Ability|GetAvatarActorfromActorInfo)))
  (bind _output_get (Variables|Default|SetCharacter%20Movement (Variables|/Script/Engine.Character|GetCharacterMovement _ascharacter)))
  (Variables|Default|SetBaseWalkSpeed (Variables|/Script/Engine.CharacterMovementComponent|GetMaxWalkSpeed _output_get))
  (if (> (Math|Vector|VectorLengthXY (Variables|/Script/Engine.MovementComponent|GetVelocity (Variables|Default|GetCharacter%20Movement))) 1e+02)
    (Ability|Tasks|WaitGameplayEvent "(TagName=\"Gameplay.CancelSprint\")" 0 true
      (:then
        (bind _returnvalue (Ability|CommitAbility))
        (if _returnvalue
          (Variables|/Script/Engine.CharacterMovementComponent|SetMaxWalkSpeed (Variables|Default|GetCharacter%20Movement) (Variables|Default|GetRunSpeed))
          (Ability|Tasks|WaitInputRelease false
            (:OnRelease
              (Ability|EndAbility)))
          (else
            (Ability|CancelAbility))))
      (:EventReceived
        (Ability|CancelAbility)))
    (else
      (Ability|CancelAbility))))

(event Ability|EventOnEndAbility
  (params (bWasCancelled :type Boolean))
  (Ability|RemoveGameplayEffectFromOwnerWithAssetTags "(GameplayTags=((TagName=\"Ability.Sprint\")))")
  (Variables|/Script/Engine.CharacterMovementComponent|SetMaxWalkSpeed (Variables|Default|GetCharacter%20Movement) (Variables|Default|GetBaseWalkSpeed)))