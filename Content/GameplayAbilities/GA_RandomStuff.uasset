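; GA_RandomStuff is a Gameplay Ability that gives the first-person character a random weapon mesh.
; On activation it picks a random entry from its Weapons array and async-loads that asset.
; When loading completes, it sets the skeletal mesh on the avatar character's Weapon component, flags the character as having a rifle and ends.
; If either the character or mesh cast fails, it stops without calling EndAbility.
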(event Ability|EventActivateAbility
  (bind _object (Utilities|AsyncLoadAsset (.OutItem (Utilities|Array|Random (Variables|Default|GetWeapons))))
    (:Completed
      (Variables|Default|SetRandom%20Item _object)
      (bind _asbp_first_person_character (Utilities|Casting|CastToBP_FirstPersonCharacter (Ability|GetAvatarActorfromActorInfo)))
      (bind _output_get (Variables|Default|SetAs%20BP%20First%20Person%20Character _asbp_first_person_character))
      (bind _asskeletal_mesh (Utilities|Casting|CastToSkeletalMesh (Variables|Default|GetRandom%20Item)))
      (Components|SkeletalMesh|SetSkeletalMeshAsset (Variables|/Script/R_D_CPP_FPS.R_D_CPP_FPSCharacter|GetWeapon _output_get) _asskeletal_mesh)
      (Class|RDCPPFPSCharacter|SetHasRifle _output_get true)
      (Ability|EndAbility))))

(event Ability|EventOnEndAbility
  (params (bWasCancelled :type Boolean)))